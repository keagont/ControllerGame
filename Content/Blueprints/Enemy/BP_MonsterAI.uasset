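; Monster AI Blueprint that roams the level, alternating random patrol moves with trips to vents.
; Three seconds after starting a patrol move, without awaiting arrival, it heads to a random VentPoint-tagged TargetPoint.
; Only on successful arrival does it turn toward the player, wait, and patrol again, with force feedback attached to its capsule in both phases.
; Pawn sensing only prints a debug message, gated by a BP_Player cast on the pawn's class.
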(event OnSeePawn(PawnSensing)
  (params (Pawn :type Pawn%20Object%20Reference))
  (Utilities|Casting|CastToBP_PlayerClass (Utilities|GetClass Pawn))
  (Development|PrintString "Player seen"))

(event Custom|VentMove
  (bind _outactors (Actor|GetAllActorsOfClasswithTag "/Script/Engine.TargetPoint" "VentPoint"))
  (AI|AIMoveTo self "0, 0, 0" (.OutItem (Utilities|Array|Random _outactors)) 5.0 false
    (:OnSuccess
      (Transformation|SetActorRotation (Math|Rotator|MakeRotator 0.0 0.0 (.yaw (Math|Rotator|FindLookatRotation (Transformation|GetActorLocation) (Transformation|GetActorLocation (Game|GetPlayerCharacter 0))))))
      (ForceFeedback|SpawnForceFeedbackAttached "/Game/Blueprints/Enemy/ForceFeedback/FF_MonsterVent.FF_MonsterVent" (Variables|Collision|GetCapsuleComponent) "None" "0, 0, 0" "0, 0, 0" "KeepRelativeOffset" false false 1.0 0.0 "/Game/Blueprints/Enemy/ForceFeedback/FF_MonsterRoam.FF_MonsterRoam")
      (Utilities|FlowControl|Delay 5.0)
      (CallFunction|PatrolRandom))))

(event Custom|PatrolRandom
  (AI|AIMoveTo self (.RandomLocation (AI|Navigation|GetRandomReachablePointinRadius (Transformation|GetActorLocation) 5e+03 0 0)) 0 5.0 false
    (:then
      (ForceFeedback|SpawnForceFeedbackAttached "/Game/Blueprints/Enemy/ForceFeedback/FF_MonsterWalk.FF_MonsterWalk" (Variables|Collision|GetCapsuleComponent) "None" "0, 0, 0" "0, 0, 0" "KeepRelativeOffset" false false 1.0 0.0 "/Game/Blueprints/Enemy/ForceFeedback/FF_MonsterRoam.FF_MonsterRoam")
      (Utilities|FlowControl|Delay 3.0)
      (CallFunction|VentMove))))

(event EventBeginPlay
  (CallFunction|PatrolRandom))

(fn ConstructionScript)